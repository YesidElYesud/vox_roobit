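; Game mode that builds a chain of floor tiles, pre-laying a batch at BeginPlay and then enabling actor spawning on tiles added afterward.
; Each new tile spawns at the previous tile's attach transform and decrements per-type distance counters, measured in tiles rather than seconds.
; At zero, a type spawns on consecutive tiles for a random run, then rerolls its gap from the spawn DataTable.
; Tick prints both counter maps for debugging.
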(event `self.ReceiveBeginPlay`
  (for _ (range -1 17)
    (`self.AddFloorTile`))
  (set `self.bIsActorSpawnActive` true)
  (`KismetSystemLibrary.PrintString` "Started spawning objects"))

(event `self.ReceiveTick`
  (params (DeltaSeconds :type "Float (single-precision)"))
  (bind _outrownames (`DataTableFunctionLibrary.GetDataTableRowNames` "/Game/DataTables/SpawnedActorsDataTable.SpawnedActorsDataTable"))
  (for _array_element _outrownames
    (bind _returnvalue (`|GetDataTableRow` "/Game/DataTables/SpawnedActorsDataTable.SpawnedActorsDataTable" _array_element)
      (:`then`
        (bind _spawnedactortype (break `/Game/DataTables/SpawnedActors_Struct` _returnvalue))
        (`KismetSystemLibrary.PrintString` (`KismetStringLibrary.Concat_StrStr` "Spawn Distance Map: " (`KismetStringLibrary.Conv_IntToString` (`BlueprintMapLibrary.Map_Find` (`self.SpawnDistanceMap`) _spawnedactortype)) " Consecutive Spawn Map: " (`KismetStringLibrary.Conv_IntToString` (`BlueprintMapLibrary.Map_Find` (`self.ConsecutiveSpawnMap`) _spawnedactortype)) " " (`|GetEnumeratorNameAsString` _spawnedactortype)) true true (struct :`G` 0.66 :`B` 1.0 :`A` 1.0) 2.0 (`|GetEnumeratorName` _spawnedactortype))))))

(fn `AddFloorTile`
  (locals (SpawnedFloorTile :type "/Game/Blueprints/BP_FloorTile Object Reference"))
  (bind _returnvalue (`|SpawnActorFromClass` "/Game/Blueprints/BP_FloorTile.BP_FloorTile_C" (`self.NextSpawnPoint`) "Undefined" "OverrideRootScale" null null))
  (bind _asbp_floor_tile (cast `/Game/Blueprints/BP_FloorTile` _returnvalue))
  (bind _output_get (set `local.SpawnedFloorTile` _asbp_floor_tile))
  (bind _attachtransform (`/Game/Blueprints/BP_FloorTile.GetAttachTransform` _output_get))
  (set `self.NextSpawnPoint` _attachtransform)
  (if (`self.bIsActorSpawnActive`)
    (bind _keys (`BlueprintMapLibrary.Map_Keys` (`self.SpawnDistanceMap`)))
    (for _array_element _keys
      (bind _bisspawnneeded (`self.IsActorSpawnNecessary` _array_element))
      (if _bisspawnneeded
        (if (not (!= (`BlueprintMapLibrary.Map_Find` (`self.ConsecutiveSpawnMap`) _array_element) 0))
          (bind _consecutivespawntimes (`self.Get Consecutive Spawn Number` _array_element))
          (`BlueprintMapLibrary.Map_Add` (`self.ConsecutiveSpawnMap`) _array_element _consecutivespawntimes))
        (`self.SpawnActor` _array_element (`local.SpawnedFloorTile`))))))

(fn `Get Consecutive Spawn Number`
  (params (Type :type "/Game/Enums/ENUM_SpawnableActors Enum" :default "NewEnumerator0"))
  (returns (ConsecutiveSpawnTimes :type Integer))
  (locals (SpawnTimes :type Integer))
  (bind _returnvalue (`|GetDataTableRow` "/Game/DataTables/SpawnedActorsDataTable.SpawnedActorsDataTable" (`KismetStringLibrary.Conv_StringToName` (`|GetEnumeratorNameAsString` Type)))
    (:`then`
      (set `local.SpawnTimes` (`KismetMathLibrary.RandomIntegerInRange` 1 (`.MaxConsecutiveSpawns_5_4DD9FBDD4E0E624CA8C3DE9A6B536841` (break `/Game/DataTables/SpawnedActors_Struct` _returnvalue)))))
    (:`RowNotFound`
      _))
  (return (`local.SpawnTimes`)))

(fn `IsActorSpawnNecessary`
  (params (Type :type "/Game/Enums/ENUM_SpawnableActors Enum" :default "NewEnumerator0"))
  (returns (bIsSpawnNeeded :type Boolean))
  (bind _spawndistancemap (`self.SpawnDistanceMap`))
  (bind _value (`BlueprintMapLibrary.Map_Find` _spawndistancemap Type))
  (bind _returnvalue (== _value 0))
  (if (not _returnvalue)
    (`BlueprintMapLibrary.Map_Add` _spawndistancemap Type (- _value 1)))
  (return _returnvalue))

(fn `SetSpawnDistance`
  (params (Type :type "/Game/Enums/ENUM_SpawnableActors Enum" :default "NewEnumerator0"))
  (bind _returnvalue (`|GetDataTableRow` "/Game/DataTables/SpawnedActorsDataTable.SpawnedActorsDataTable" (`KismetStringLibrary.Conv_StringToName` (`|GetEnumeratorNameAsString` Type)))
    (:`then`
      (bind (_spawnedactortype _maxconsecutivespawns _mintimebetweenspawn _maxtimebetweenspawn) (break `/Game/DataTables/SpawnedActors_Struct` _returnvalue))
      (`BlueprintMapLibrary.Map_Add` (`self.SpawnDistanceMap`) _spawnedactortype (`KismetMathLibrary.RandomIntegerInRange` _mintimebetweenspawn _maxtimebetweenspawn)))))

(fn `SpawnActor`
  (params (Type :type "/Game/Enums/ENUM_SpawnableActors Enum" :default "NewEnumerator0") (FloorTile :type "/Game/Blueprints/BP_FloorTile Object Reference"))
  (locals (FloorTileRef :type "/Game/Blueprints/BP_FloorTile Object Reference") (ActorType :type "/Game/Enums/ENUM_SpawnableActors Enum"))
  (bind _floortileref (`local.FloorTileRef`))
  (bind _consecutivespawnmap (`self.ConsecutiveSpawnMap`))
  (bind _actortype (`local.ActorType`))
  (bind _actortype_2 (`local.ActorType`))
  (bind _output_get (set `local.ActorType` Type))
  (set `local.FloorTileRef` FloorTile)
  (bind _returnvalue (`|GetDataTableRow` "/Game/DataTables/SpawnedActorsDataTable.SpawnedActorsDataTable" (`KismetStringLibrary.Conv_StringToName` (`|GetEnumeratorNameAsString` _output_get)))
    (:`then`
      (bind _spawnpoints (`/Game/Blueprints/BP_FloorTile.GetValidActorSpawnPoint` _floortileref))
      (`|SpawnActorFromClass` (`.ActorToSpawn_12_A84AAC3D46BF6142DCC836A14965EA40` (break `/Game/DataTables/SpawnedActors_Struct` _returnvalue)) (`KismetMathLibrary.MakeTransform` (+ (.location _spawnpoints) (.location (`self.GetTransform` _floortileref))) (.rotation (`self.GetTransform` _floortileref)) (.scale (`self.GetTransform` _floortileref))) "Undefined" "OverrideRootScale" null null)
      (`BlueprintMapLibrary.Map_Add` _consecutivespawnmap _actortype_2 (- (`BlueprintMapLibrary.Map_Find` _consecutivespawnmap _actortype_2) 1))
      (if (== (`BlueprintMapLibrary.Map_Find` (`self.ConsecutiveSpawnMap`) _actortype) 0)
        (`self.SetSpawnDistance` _actortype)))))

(fn `StartTimers`
  (bind _outrownames (`DataTableFunctionLibrary.GetDataTableRowNames` "/Game/DataTables/SpawnedActorsDataTable.SpawnedActorsDataTable"))
  (for _array_element _outrownames
    (bind _returnvalue (`|GetDataTableRow` "/Game/DataTables/SpawnedActorsDataTable.SpawnedActorsDataTable" _array_element)
      (:`then`
        (bind _spawnedactortype (break `/Game/DataTables/SpawnedActors_Struct` _returnvalue))
        (`BlueprintMapLibrary.Map_Add` (`self.SpawnDistanceMap`) _spawnedactortype)
        (`self.SetSpawnDistance` _spawnedactortype)))))

(fn `UserConstructionScript`
  (bind _outrownames (`DataTableFunctionLibrary.GetDataTableRowNames` "/Game/DataTables/SpawnedActorsDataTable.SpawnedActorsDataTable"))
  (for _array_element _outrownames
    (bind _returnvalue (`|GetDataTableRow` "/Game/DataTables/SpawnedActorsDataTable.SpawnedActorsDataTable" _array_element)
      (:`then`
        (`BlueprintMapLibrary.Map_Add` (`self.ConsecutiveSpawnMap`) (`.SpawnedActorType_2_CCABCFCF4E47532B8C03E0AFA0F30CF8` (break `/Game/DataTables/SpawnedActors_Struct` _returnvalue)) 1))))
  (`self.StartTimers`))