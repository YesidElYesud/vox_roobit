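; BP_Chile is a spawned chili actor that triggers the player rabbit's Chilesito effect through its collision behavior.
; On BeginPlay it runs the parent logic, then sets the inherited Sphere1 component to the Chile mesh and scales it down.
; Its ExecuteCollisionBehavior event casts player character 0 to BP_Conejo and calls Chilesito, leaving the effect itself to that character.
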(event `self.ReceiveBeginPlay`
  (bind _sphere1 (`self.Sphere1`))
  (`parent.ReceiveBeginPlay`)
  (`StaticMeshComponent.SetStaticMesh` _sphere1 "/Game/Meshs/chile.chile")
  (`SceneComponent.SetRelativeScale3D` _sphere1 (0.02 0.02 0.02)))

(event `/Game/Blueprints/Interfaces/BPI_ExecuteCollisionAction.ExecuteCollisionBehavior`
  (bind _asbp_conejo (cast `/Game/Blueprints/Blueprints/BP_Conejo` (`GameplayStatics.GetPlayerCharacter` 0)))
  (`/Game/Blueprints/Blueprints/BP_Conejo.Chilesito` _asbp_conejo))

(fn `UserConstructionScript`
  (`parent.UserConstructionScript`))