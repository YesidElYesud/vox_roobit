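; BP_Rabanos is a spawned radish actor that awards the player a point through its collision behavior.
; On BeginPlay it runs the parent logic, then sets the inherited Sphere1 component to the Rabano mesh and scales it down.
; Its ExecuteCollisionBehavior event casts the game instance to InstanciaDelJuego and increments Puntos, leaving overlap detection outside this graph.
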(event `self.ReceiveBeginPlay`
  (bind _sphere1 (`self.Sphere1`))
  (`parent.ReceiveBeginPlay`)
  (`StaticMeshComponent.SetStaticMesh` _sphere1 "/Game/Meshs/rabano.rabano")
  (`SceneComponent.SetRelativeScale3D` _sphere1 (0.02 0.02 0.02)))

(event `/Game/Blueprints/Interfaces/BPI_ExecuteCollisionAction.ExecuteCollisionBehavior`
  (`|ExecutionSequence`
    (:`then_0`
      (bind _asinstancia_del_juego (cast `/Game/Blueprints/Blueprints/InstanciaDelJuego` (`GameplayStatics.GetGameInstance`)))
      (`/Engine/EditorBlueprintResources/StandardMacros.IncrementInt` (`/Game/Blueprints/Blueprints/InstanciaDelJuego.Puntos` _asinstancia_del_juego)))))

(fn `UserConstructionScript`
  (`parent.UserConstructionScript`))