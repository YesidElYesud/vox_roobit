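; BP_PiedraMal2 is a spawned pickup-style actor that appears as a small mushroom and gives the rabbit player a temporary speed change.
; BeginPlay runs the parent logic, then swaps Sphere1's mesh to Hongo2 and shrinks it.
; Its ExecuteCollisionBehavior event calls Inmune on the player's BP_Conejo, raises max walk speed, then sets a lower fixed speed after a five-second delay.
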(event `self.ReceiveBeginPlay`
  (bind _sphere1 (`self.Sphere1`))
  (`parent.ReceiveBeginPlay`)
  (`StaticMeshComponent.SetStaticMesh` _sphere1 "/Game/Meshs/hongo2.hongo2")
  (`SceneComponent.SetRelativeScale3D` _sphere1 (0.02 0.02 0.02)))

(event `/Game/Blueprints/Interfaces/BPI_ExecuteCollisionAction.ExecuteCollisionBehavior`
  (`|ExecutionSequence`
    (:`then_1`
      (bind _asbp_conejo (cast `/Game/Blueprints/Blueprints/BP_Conejo` (`GameplayStatics.GetPlayerCharacter` 0)))
      (`/Game/Blueprints/Blueprints/BP_Conejo.Inmune` _asbp_conejo)
      (bind _charactermovement (`Character.CharacterMovement` _asbp_conejo))
      (set `CharacterMovementComponent.MaxWalkSpeed` 900.0 _charactermovement)
      (`KismetSystemLibrary.Delay` 5.0)
      (set `CharacterMovementComponent.MaxWalkSpeed` 500.0 _charactermovement))))

(fn `UserConstructionScript`
  (`parent.UserConstructionScript`))