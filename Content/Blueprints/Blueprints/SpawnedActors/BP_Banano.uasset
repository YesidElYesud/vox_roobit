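; BP_Banano is a banana power-up pickup that awards points and triggers immunity on the rabbit player.
; On BeginPlay it runs the parent logic, then sets the Sphere1 component to a scaled-down banana mesh.
; Its ExecuteCollisionBehavior event adds to Puntos on the game instance, calls Inmune on BP_Conejo and plays two 2D sounds, one pitched up.
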(event `self.ReceiveBeginPlay`
  (bind _sphere1 (`self.Sphere1`))
  (`parent.ReceiveBeginPlay`)
  (`StaticMeshComponent.SetStaticMesh` _sphere1 "/Game/Meshs/banano.banano")
  (`SceneComponent.SetRelativeScale3D` _sphere1 (0.02 0.02 0.02)))

(event `/Game/Blueprints/Interfaces/BPI_ExecuteCollisionAction.ExecuteCollisionBehavior`
  (`|ExecutionSequence`
    (:`then_0`
      (bind _asinstancia_del_juego (cast `/Game/Blueprints/Blueprints/InstanciaDelJuego` (`GameplayStatics.GetGameInstance`)))
      (set `/Game/Blueprints/Blueprints/InstanciaDelJuego.Puntos` (+ 3 (`/Game/Blueprints/Blueprints/InstanciaDelJuego.Puntos` _asinstancia_del_juego)) _asinstancia_del_juego))
    (:`then_1`
      (bind _asbp_conejo (cast `/Game/Blueprints/Blueprints/BP_Conejo` (`GameplayStatics.GetPlayerCharacter` 0)))
      (`/Game/Blueprints/Blueprints/BP_Conejo.Inmune` _asbp_conejo))
    (:`then_2`
      (`GameplayStatics.PlaySound2D` "/Game/Sound/powerup_Cue.powerup_Cue" 1.0 1.0 0.0 null null)
      (`GameplayStatics.PlaySound2D` (`self.Sound`) 1.0 1.8 0.0 null null))))

(fn `UserConstructionScript`
  (`parent.UserConstructionScript`))