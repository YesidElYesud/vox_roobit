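; BP_HongoAzul is a blue mushroom pickup that awards points and boosts the rabbit player character.
; BeginPlay assigns the Hongo2 mesh to Sphere1 at a tiny scale.
; ExecuteCollisionBehavior runs chained increments starting from the game instance's Puntos, then calls Inmune on BP_Conejo and raises its walk speed, restoring a fixed speed after a delay.
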(event `self.ReceiveBeginPlay`
  (bind _sphere1 (`self.Sphere1`))
  (`parent.ReceiveBeginPlay`)
  (`StaticMeshComponent.SetStaticMesh` _sphere1 "/Game/Meshs/hongo2.hongo2")
  (`SceneComponent.SetRelativeScale3D` _sphere1 (0.02 0.02 0.02)))

(event `/Game/Blueprints/Interfaces/BPI_ExecuteCollisionAction.ExecuteCollisionBehavior`
  (`|ExecutionSequence`
    (:`then_0`
      (bind _asinstancia_del_juego (cast `/Game/Blueprints/Blueprints/InstanciaDelJuego` (`GameplayStatics.GetGameInstance`)))
      (bind _result (`/Engine/EditorBlueprintResources/StandardMacros.IncrementInt` (`/Game/Blueprints/Blueprints/InstanciaDelJuego.Puntos` _asinstancia_del_juego))
        (:`  `
          (bind _result_2 (`/Engine/EditorBlueprintResources/StandardMacros.IncrementInt` _result)
            (:`  `
              (bind _result_3 (`/Engine/EditorBlueprintResources/StandardMacros.IncrementInt` _result_2)
                (:`  `
                  (bind _result_4 (`/Engine/EditorBlueprintResources/StandardMacros.IncrementInt` _result_3)
                    (:`  `
                      (bind _result_5 (`/Engine/EditorBlueprintResources/StandardMacros.IncrementInt` _result_4)
                        (:`  `
                          (`/Engine/EditorBlueprintResources/StandardMacros.IncrementInt` _result_5))))))))))))
    (:`then_1`
      (bind _asbp_conejo (cast `/Game/Blueprints/Blueprints/BP_Conejo` (`GameplayStatics.GetPlayerCharacter` 0)))
      (`/Game/Blueprints/Blueprints/BP_Conejo.Inmune` _asbp_conejo)
      (bind _charactermovement (`Character.CharacterMovement` _asbp_conejo))
      (set `CharacterMovementComponent.MaxWalkSpeed` 900.0 _charactermovement)
      (`KismetSystemLibrary.Delay` 5.0)
      (set `CharacterMovementComponent.MaxWalkSpeed` 500.0 _charactermovement))))

(fn `UserConstructionScript`
  (`parent.UserConstructionScript`))