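; Floor tile for an endlessly extending track: when BP_Conejo overlaps its box, it asks the game mode for another tile, then destroys itself after a delay.
; An arrow supplies the attach transform for chaining tiles.
; Construction caches spawn points and adds a randomly rotated child-actor blocker at one of twelve root points.
; GetValidActorSpawnPoint randomly retries three actor points until one is free, then marks it used.
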(event `self.Box.OnComponentBeginOverlap`
  (params (OverlappedComponent :type "PrimitiveComponent Object Reference") (OtherActor :type "Actor Object Reference") (OtherComp :type "PrimitiveComponent Object Reference") (OtherBodyIndex :type Integer) (bFromSweep :type Boolean) (SweepResult :type "HitResult Structure (by ref)"))
  (cast `/Game/Blueprints/Blueprints/BP_Conejo` OtherActor)
  (bind _asbp_conejo_game_mode (cast `/Game/Blueprints/Blueprints/BP_ConejoGameMode` (`GameplayStatics.GetGameMode`)))
  (`/Game/Blueprints/Blueprints/BP_ConejoGameMode.AddFloorTile` _asbp_conejo_game_mode)
  (`KismetSystemLibrary.Delay` 4.0)
  (`self.K2_DestroyActor`))

(fn `GetAttachTransform`
  (returns (AttachTransform :type "Transform Structure"))
  (return (`SceneComponent.K2_GetComponentToWorld` (`self.Arrow`))))

(fn `GetValidActorSpawnPoint`
  (returns (SpawnPoints :type "Transform Structure"))
  (locals (bPositionFound :type Boolean) (RandomIndex :type Integer))
  (bind _randomindex (`local.RandomIndex`))
  (while (not (`local.bPositionFound`))
    (set `local.RandomIndex` (`KismetMathLibrary.RandomIntegerInRange` 0 2))
    (if (not (`BlueprintMapLibrary.Map_Find` (`self.ActorSpawnPointValue`) _randomindex))
      (set `local.bPositionFound` true)))
  (`BlueprintMapLibrary.Map_Add` (`self.ActorSpawnPointValue`) _randomindex true)
  (return (`|GetArrayItem` (`self.ActorSpawnPoints`) _randomindex)))

(fn `SetActorSpawnPoints`
  (bind _output_get (set `self.ActorSpawnPoints` (`|MakeArray` (`SceneComponent.GetRelativeTransform` (`self.ActorSpawnPoint 1`)) (`SceneComponent.GetRelativeTransform` (`self.ActorSpawnPoint 2`)) (`SceneComponent.GetRelativeTransform` (`self.ActorSpawnPoint 3`)))))
  (for (_ _array_index) _output_get
    (`BlueprintMapLibrary.Map_Add` (`self.ActorSpawnPointValue`) _array_index)))

(fn `SetRootSpawnPoints`
  (set `self.RootSpawnPoints` (`|MakeArray` (`SceneComponent.GetRelativeTransform` (`self.p1`)) (`SceneComponent.GetRelativeTransform` (`self.p2`)) (`SceneComponent.GetRelativeTransform` (`self.p3`)) (`SceneComponent.GetRelativeTransform` (`self.p4`)) (`SceneComponent.GetRelativeTransform` (`self.p5`)) (`SceneComponent.GetRelativeTransform` (`self.p6`)) (`SceneComponent.GetRelativeTransform` (`self.p7`)) (`SceneComponent.GetRelativeTransform` (`self.p8`)) (`SceneComponent.GetRelativeTransform` (`self.p9`)) (`SceneComponent.GetRelativeTransform` (`self.p10`)) (`SceneComponent.GetRelativeTransform` (`self.p11`)) (`SceneComponent.GetRelativeTransform` (`self.p12`)))))

(fn `SpawnBlocker`
  (bind _output (`|GetArrayItem` (`self.RootSpawnPoints`) (`self.RootSpawnPointIndex`)))
  (set `self.RootSpawnPointIndex` (`KismetMathLibrary.RandomIntegerInRange` 0 11))
  (`AddComponent|NODE_AddChildActorComponent-0` :`RelativeTransform` (`KismetMathLibrary.MakeTransform` (.location _output) (`KismetMathLibrary.MakeRotator` (`KismetMathLibrary.RandomFloatInRange` 0.0 180.0) (`KismetMathLibrary.RandomFloatInRange` 0.0 180.0) (`KismetMathLibrary.RandomFloatInRange` 0.0 180.0)) (.scale _output))))

(fn `UserConstructionScript`
  (`self.SetActorSpawnPoints`)
  (`self.SetRootSpawnPoints`)
  (`self.SpawnBlocker`))